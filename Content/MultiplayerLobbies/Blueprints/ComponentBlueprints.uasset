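; Function library of helpers for projectile stats, operating on the ProjectileInfo struct.
; AddBounces, AddSpeed and AddDamage each return a rebuilt struct with one value increased, with damage changed inside the nested DamageInfo.
; Projectile properties are packed into an integer bitmask, tested and toggled by HasProjectileProperty and SetProjectileProperty.
; Both derive the bit from the enum index as a power of two through ConvertIntegerToBitwise.
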(fn `Add Damage`
  (params (ProjectileInfo :type "/Game/MultiplayerLobbies/Blueprints/DamageSystem/ProjectileInfo Structure") (Damage :type "Float (double-precision)"))
  (returns (NewProjectileInfo :type "/Game/MultiplayerLobbies/Blueprints/DamageSystem/ProjectileInfo Structure"))
  (bind (_damageinfo _speed _bounces _projectileflagproperties) (break `/Game/MultiplayerLobbies/Blueprints/DamageSystem/ProjectileInfo` ProjectileInfo))
  (bind (_amount _damagetype _damageresponse _shoulddamageinvinvible _canbeblocked) (break `/Game/MultiplayerLobbies/Blueprints/DamageSystem/DamageInfo` _damageinfo))
  (return (make `/Game/MultiplayerLobbies/Blueprints/DamageSystem/ProjectileInfo` (make `/Game/MultiplayerLobbies/Blueprints/DamageSystem/DamageInfo` (+ _amount Damage) _damagetype _damageresponse _shoulddamageinvinvible _canbeblocked) _speed _bounces _projectileflagproperties)))

(fn `AddBounces`
  (params (ProjectileInfo :type "/Game/MultiplayerLobbies/Blueprints/DamageSystem/ProjectileInfo Structure") (Bounces :type Integer))
  (returns (NewProjectileInfo :type "/Game/MultiplayerLobbies/Blueprints/DamageSystem/ProjectileInfo Structure"))
  (bind (_damageinfo _speed _bounces _projectileflagproperties) (break `/Game/MultiplayerLobbies/Blueprints/DamageSystem/ProjectileInfo` ProjectileInfo))
  (return (make `/Game/MultiplayerLobbies/Blueprints/DamageSystem/ProjectileInfo` _damageinfo _speed (+ _bounces Bounces) _projectileflagproperties)))

(fn `AddSpeed`
  (params (ProjectileInfo :type "/Game/MultiplayerLobbies/Blueprints/DamageSystem/ProjectileInfo Structure") (Speed :type "Float (double-precision)"))
  (returns (NewProjectileInfo :type "/Game/MultiplayerLobbies/Blueprints/DamageSystem/ProjectileInfo Structure"))
  (bind (_damageinfo _speed _bounces _projectileflagproperties) (break `/Game/MultiplayerLobbies/Blueprints/DamageSystem/ProjectileInfo` ProjectileInfo))
  (return (make `/Game/MultiplayerLobbies/Blueprints/DamageSystem/ProjectileInfo` _damageinfo (+ _speed Speed) _bounces _projectileflagproperties)))

(fn `Convert Integer to Bitwise`
  (params (EnumInteger :type Integer))
  (returns (BitwiseInteger :type Integer))
  (return (`KismetMathLibrary.FFloor` (`KismetMathLibrary.MultiplyMultiply_FloatFloat` 2.0 (`KismetMathLibrary.Conv_IntToDouble` EnumInteger)))))

(fn `HasProjectileProperty`
  (params (Properties :type Integer) (`Projectile Property` :type "/Game/MultiplayerLobbies/Blueprints/DamageSystem/ProjectileFlagProperties Enum" :default "NewEnumerator2"))
  (returns (`Has Property` :type Boolean))
  (return (`KismetMathLibrary.Conv_IntToBool` (`KismetMathLibrary.And_IntInt` Properties (`self.Convert Integer to Bitwise` (`KismetMathLibrary.Conv_ByteToInt` `Projectile Property`))))))

(fn `SetProjectileProperty`
  (params (ProjectileInfo :type "/Game/MultiplayerLobbies/Blueprints/DamageSystem/ProjectileInfo Structure") (FlagProperty :type "/Game/MultiplayerLobbies/Blueprints/DamageSystem/ProjectileFlagProperties Enum" :default "NewEnumerator4") (SetValue :type Boolean :default true))
  (returns (NewProjectileInfo :type "/Game/MultiplayerLobbies/Blueprints/DamageSystem/ProjectileInfo Structure"))
  (locals (ProjectileProperties :type Integer))
  (bind (_damageinfo _speed _bounces _projectileflagproperties) (break `/Game/MultiplayerLobbies/Blueprints/DamageSystem/ProjectileInfo` ProjectileInfo))
  (if SetValue
    (set `local.ProjectileProperties` (`KismetMathLibrary.Or_IntInt` (`self.Convert Integer to Bitwise` (`KismetMathLibrary.Conv_ByteToInt` FlagProperty)) _projectileflagproperties))
    (else
      (set `local.ProjectileProperties` (`KismetMathLibrary.And_IntInt` (`KismetMathLibrary.Not_Int` (`self.Convert Integer to Bitwise` (`KismetMathLibrary.Conv_ByteToInt` FlagProperty))) _projectileflagproperties))))
  (return (make `/Game/MultiplayerLobbies/Blueprints/DamageSystem/ProjectileInfo` _damageinfo _speed _bounces (`local.ProjectileProperties`))))