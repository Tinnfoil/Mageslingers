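; Function library for building modular weapons and pickupable items from item data.
; ConstructWeaponMesh socket-attaches head and tail meshes to the body, then adds gem meshes parsed from a delimited gem string, which SetGemsForComponent edits.
; Each part's optional logic class becomes a component on the character, and GenerateProjectileInfo chains those components to modify projectile info.
; Helpers cover bitmask item-type checks, child cleanup and string joining.
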(fn `CombineStringsWithSeparator`
  (params (List :type "Array of String") (Separator :type String))
  (returns (OutputString :type String))
  (locals (Result :type String) (Seperator :type String))
  (bind _result (`local.Result`))
  (set `local.Seperator` Separator)
  (if (> (`KismetArrayLibrary.Array_Length` List) 0)
    (for (_array_element _array_index) List
      (if (!= _array_index (- (`KismetArrayLibrary.Array_Length` List) 1))
        (set `local.Result` (`KismetStringLibrary.Concat_StrStr` _result (`KismetStringLibrary.Concat_StrStr` _array_element (`local.Seperator`))))
        (else
          (set `local.Result` (`KismetStringLibrary.Concat_StrStr` _result _array_element)))))
    (return (`local.Result`))
    (else
      (return (`local.Result`)))))

(fn `Construct Pickupable Item`
  (params (`Pickupable Item` :type "/Game/MultiplayerLobbies/Blueprints/BP_PickupableObject Object Reference") (ItemData :type "/Game/MultiplayerLobbies/Datatables/BaseItemData Structure"))
  (bind _basemesh (`BaseObject.BaseMesh` `Pickupable Item`))
  (`StaticMeshComponent.SetStaticMesh` _basemesh (`.StaticMesh_10_603EC9A743521CB4AF0D318101D7906B` (break `/Game/MultiplayerLobbies/Datatables/BaseItemData` ItemData)))
  (`PrimitiveComponent.SetSimulatePhysics` _basemesh true))

(fn `Construct Weapon Mesh`
  (params (BaseMesh :type "StaticMeshComponent Object Reference") (WeaponData :type "/Game/MultiplayerLobbies/Datatables/WeaponItemData Structure") (Target :type "Actor Object Reference") (ComponentLogicParent :type "SceneComponent Object Reference"))
  (returns (ItemRowData :type "Array of String"))
  (locals (TargetActor :type "Actor Object Reference") (BaseMeshComponent :type "StaticMeshComponent Object Reference") (TargetMesh :type "StaticMeshComponent Object Reference") (HeadMesh :type "StaticMeshComponent Object Reference") (TailMesh :type "StaticMeshComponent Object Reference") (GemSocketNum :type Integer) (`Collision Profile` :type Name) (CurrPieceName :type String) (CurrGemName :type String) (ReturnGemData :type "Array of String") (LogicComponent :type "SceneComponent Object Reference") (CharacterBP :type "/Game/MultiplayerLobbies/Blueprints/BaseCharacter_BP Object Reference"))
  (bind (_headpiece _mainbody _tailpiece _gems) (break `/Game/MultiplayerLobbies/Datatables/WeaponItemData` WeaponData))
  (bind _returngemdata (`local.ReturnGemData`))
  (bind _returngemdata_2 (`local.ReturnGemData`))
  (bind _returngemdata_3 (`local.ReturnGemData`))
  (bind _asbase_character_bp (cast `/Game/MultiplayerLobbies/Blueprints/BaseCharacter_BP` Target)
    (:`then`
      (set `local.LogicComponent` ComponentLogicParent)
      (set `local.CharacterBP` _asbase_character_bp))
    (:`CastFailed`
      _))
  (`self.DestroyAllChildren` BaseMesh)
  (set `local.TargetActor` Target)
  (set `local.BaseMeshComponent` BaseMesh)
  (set `local.Collision Profile` (`PrimitiveComponent.GetCollisionProfileName` BaseMesh))
  ;[1 1 1] Body
  (`self.Set Weapon Component Mesh` BaseMesh _mainbody)
  (`self.InitializeComponentLogic` (`local.LogicComponent`) (`local.CharacterBP`) (`.ItemData_2_AB890E3145ADAEB69815B3B9B749E7DE` (break `/Game/MultiplayerLobbies/Datatables/ComponentData` _mainbody)))
  ;[1 1 1] Head
  (bind _returnvalue (`|AddComponentByClass` :`self` (`local.TargetActor`) :`Class` "/Script/Engine.StaticMeshComponent"))
  (set `local.HeadMesh` _returnvalue)
  (`self.Set Weapon Component Mesh` _returnvalue _headpiece)
  (`self.InitializeComponentLogic` (`local.LogicComponent`) (`local.CharacterBP`) (`.ItemData_2_AB890E3145ADAEB69815B3B9B749E7DE` (break `/Game/MultiplayerLobbies/Datatables/ComponentData` _headpiece)))
  (`PrimitiveComponent.SetCollisionProfileName` _returnvalue (`local.Collision Profile`) true)
  (`SceneComponent.K2_AttachToComponent` _returnvalue (`local.BaseMeshComponent`) "Head" "KeepRelative" "KeepRelative" "KeepRelative" true)
  ;[1 1 1] Tail
  (bind _returnvalue_2 (`|AddComponentByClass` :`self` (`local.TargetActor`) :`Class` "/Script/Engine.StaticMeshComponent"))
  (set `local.TailMesh` _returnvalue_2)
  (`self.Set Weapon Component Mesh` _returnvalue_2 _tailpiece)
  (`self.InitializeComponentLogic` (`local.LogicComponent`) (`local.CharacterBP`) (`.ItemData_2_AB890E3145ADAEB69815B3B9B749E7DE` (break `/Game/MultiplayerLobbies/Datatables/ComponentData` _tailpiece)))
  (`PrimitiveComponent.SetCollisionProfileName` _returnvalue_2 (`local.Collision Profile`) true)
  (`SceneComponent.K2_AttachToComponent` _returnvalue_2 (`local.BaseMeshComponent`) "Tail" "KeepRelative" "KeepRelative" "KeepRelative" true)
  (for _array_element (`KismetStringLibrary.ParseIntoArray` _gems ";")
    (bind _returnvalue_3 (`KismetStringLibrary.ParseIntoArray` _array_element ":"))
    (bind _output (`|GetArrayItem` _returnvalue_3))
    (`KismetSystemLibrary.LogString` (`KismetStringLibrary.Concat_StrStr` "#" _output))
    (set `local.CurrPieceName` _output)
    (for (_array_element_2 _array_index) (`KismetStringLibrary.ParseIntoArray` (`|GetArrayItem` _returnvalue_3 1) ",")
      (set `local.CurrGemName` _array_element_2)
      (set `local.GemSocketNum` (+ _array_index 1))
      (bind _returnvalue_4 (`KismetStringLibrary.Conv_StringToName` _array_element_2))
      (`|GetDataTableRow` "/Game/MultiplayerLobbies/Datatables/DB_GemDatabase.DB_GemDatabase" _returnvalue_4
        (:`then`
          (`KismetSystemLibrary.LogString` (`KismetStringLibrary.Conv_NameToString` _returnvalue_4))
          (switch `string` _output
            (:`Head`
              (set `local.TargetMesh` (`local.HeadMesh`))
              (`KismetArrayLibrary.Array_Set` _returngemdata_3 0 (`KismetStringLibrary.Concat_StrStr` (`KismetStringLibrary.Concat_StrStr` (`|GetArrayItem` _returngemdata_3) (`local.CurrGemName`)) ",")))
            (:`Body`
              (set `local.TargetMesh` (`local.BaseMeshComponent`))
              (`KismetArrayLibrary.Array_Set` _returngemdata_2 1 (`KismetStringLibrary.Concat_StrStr` (`KismetStringLibrary.Concat_StrStr` (`|GetArrayItem` _returngemdata_2 1) (`local.CurrGemName`)) ",")))
            (:`Tail`
              (set `local.TargetMesh` (`local.TailMesh`))
              (`KismetArrayLibrary.Array_Set` _returngemdata 2 (`KismetStringLibrary.Concat_StrStr` (`KismetStringLibrary.Concat_StrStr` (`|GetArrayItem` _returngemdata 2) (`local.CurrGemName`)) ","))))
          (bind _returnvalue_5 (`|GetDataTableRow` "/Game/MultiplayerLobbies/Datatables/DB_GemDatabase.DB_GemDatabase" (`KismetStringLibrary.Conv_StringToName` (`local.CurrGemName`)))
            (:`then`
              (bind _returnvalue_6 (`|AddComponentByClass` :`self` (`local.TargetActor`) :`Class` "/Script/Engine.StaticMeshComponent"))
              (bind _itemdata (break `/Game/MultiplayerLobbies/Datatables/GemData` _returnvalue_5))
              (`self.InitializeComponentLogic` (`local.LogicComponent`) (`local.CharacterBP`) _itemdata)
              (`StaticMeshComponent.SetStaticMesh` _returnvalue_6 (`.StaticMesh_10_603EC9A743521CB4AF0D318101D7906B` (break `/Game/MultiplayerLobbies/Datatables/BaseItemData` _itemdata)))
              (`PrimitiveComponent.SetCollisionEnabled` _returnvalue_6 "NoCollision")
              (`SceneComponent.K2_AttachToComponent` _returnvalue_6 (`local.TargetMesh`) (`KismetStringLibrary.Conv_StringToName` (`KismetStringLibrary.Concat_StrStr` "Gem Socket " (`KismetStringLibrary.Conv_IntToString` (`local.GemSocketNum`)))) "KeepRelative" "KeepRelative" "KeepRelative" true)))))))
  (return (`local.ReturnGemData`)))

(fn `DestroyAllChildren`
  (params (Target :type "SceneComponent Object Reference"))
  (returns (Success :type Boolean))
  (`/Engine/EditorBlueprintResources/StandardMacros.IsValid` Target
    (:`Is Valid`
      (while (> (`SceneComponent.GetNumChildrenComponents` Target) 0)
        (`ActorComponent.K2_DestroyComponent` (`SceneComponent.GetChildComponent` Target 0)))
      (return true))))

(fn `GenerateProjectileInfo`
  (params (BaseProjectileInfo :type "/Game/MultiplayerLobbies/Blueprints/DamageSystem/ProjectileInfo Structure") (ComponentLogics :type "Array of /Game/MultiplayerLobbies/Blueprints/WeaponComponents/ComponentLogic Object Reference"))
  (returns (ProjectileInfo :type "/Game/MultiplayerLobbies/Blueprints/DamageSystem/ProjectileInfo Structure"))
  (locals (CurrentProjectileInfo :type "/Game/MultiplayerLobbies/Blueprints/DamageSystem/ProjectileInfo Structure"))
  (set `local.CurrentProjectileInfo` BaseProjectileInfo)
  (for _array_element ComponentLogics
    (bind _new_projectile_info (`/Game/MultiplayerLobbies/Blueprints/WeaponComponents/ComponentLogic.ApplyComponentEffectProjectile` _array_element (`local.CurrentProjectileInfo`)))
    (set `local.CurrentProjectileInfo` _new_projectile_info))
  (return (`local.CurrentProjectileInfo`)))

(fn `Get Socket Offset`
  (params (`Static Mesh` :type "StaticMeshComponent Object Reference") (SocketName :type Name))
  (returns (Offset :type "Transform Structure"))
  (return (`SceneComponent.GetSocketTransform` `Static Mesh` SocketName "RTS_Actor")))

(fn `Initialize Weapon Component`
  (params (`Weapon Component` :type "WeaponComponentObject Object Reference") (ItemComponentData :type "/Game/MultiplayerLobbies/Datatables/ComponentData Structure"))
  (`self.Set Weapon Component Mesh` (`BaseObject.BaseMesh` `Weapon Component`) ItemComponentData))

(fn `InitializeComponentLogic`
  (params (ParentComponent :type "SceneComponent Object Reference") (TargetActor :type "/Game/MultiplayerLobbies/Blueprints/BaseCharacter_BP Object Reference") (ItemData :type "/Game/MultiplayerLobbies/Datatables/BaseItemData Structure"))
  (bind (_name _staticmesh _icon _type _objectreference _componentlogic) (break `/Game/MultiplayerLobbies/Datatables/BaseItemData` ItemData))
  (`/Engine/EditorBlueprintResources/StandardMacros.IsValid` ParentComponent
    (:`Is Valid`
      (if (!= _componentlogic null)
        (bind _returnvalue (`|AddComponentByClass` :`self` TargetActor :`Class` _componentlogic :`BaseCharacter` TargetActor))
        (`SceneComponent.K2_AttachToComponent` _returnvalue ParentComponent "None" "KeepRelative" "KeepRelative" "KeepRelative" true)
        (`KismetArrayLibrary.Array_Add` (`/Game/MultiplayerLobbies/Blueprints/BaseCharacter_BP.ComponentLogics` TargetActor) _returnvalue)
        (else
          (return))))
    (:`Is Not Valid`
      (return))))

(fn `Is Valid Item Type`
  (params (ValidItemTypes :type Integer) (ItemType :type "/Game/MultiplayerLobbies/Datatables/WeaponComponentType Enum" :default "NewEnumerator0"))
  (returns (IsValidItemType :type Boolean))
  (locals (Base2 :type Integer) (Base2_0 :type Integer64))
  (return (`KismetMathLibrary.Conv_IntToBool` (`KismetMathLibrary.And_IntInt` ValidItemTypes (`KismetMathLibrary.FFloor` (`KismetMathLibrary.MultiplyMultiply_FloatFloat` 2.0 (`KismetMathLibrary.Conv_IntToDouble` (`KismetMathLibrary.Conv_ByteToInt` ItemType))))))))

(fn `Set Gems For Component`
  (params (ComponentType :type "/Game/MultiplayerLobbies/Datatables/WeaponComponentType Enum" :default "NewEnumerator0") (Gems :type String) (`Socket Index` :type Integer) (`Gem Name` :type String))
  (returns (GemData :type String))
  (locals (ItemType :type "/Game/MultiplayerLobbies/Datatables/WeaponComponentType Enum") (Index :type Integer) (GemName :type String) (NewGemArray :type "Array of String") (TempStringArray :type "Array of String"))
  (bind _returnvalue (`KismetStringLibrary.ParseIntoArray` Gems ";"))
  (bind _index (`local.Index`))
  (set `local.ItemType` ComponentType)
  (set `local.Index` `Socket Index`)
  (set `local.GemName` `Gem Name`)
  (set `local.NewGemArray` _returnvalue)
  (for (_array_element _array_index) _returnvalue
    (bind _returnvalue_2 (`KismetStringLibrary.ParseIntoArray` _array_element ":"))
    (bind _output (`|GetArrayItem` _returnvalue_2))
    (switch `string` _output
      (:`Body`
        (if (`|EnumEquality` (`local.ItemType`) "NewEnumerator0")
          (bind _output_get (set `local.TempStringArray` (`KismetStringLibrary.ParseIntoArray` (`|GetArrayItem` _returnvalue_2 1) ",") :!label _label))
          (bind _returnvalue_3 (<= (`KismetArrayLibrary.Array_Length` _output_get) (`local.Index`)))
          (if _returnvalue_3
            (while _returnvalue_3
              (`KismetArrayLibrary.Array_Add` (`local.TempStringArray`) "Null")))
          (for (_ _array_index_2) (`local.TempStringArray`)
            (if (== _array_index_2 _index)
              (`KismetArrayLibrary.Array_Set` (`local.TempStringArray`) _index (`local.GemName`))
              (break)))
          (bind _outputstring (`self.CombineStringsWithSeparator` (`local.TempStringArray`) ","))
          (`KismetArrayLibrary.Array_Set` (`local.NewGemArray`) _array_index (`KismetStringLibrary.Concat_StrStr` (`KismetStringLibrary.Concat_StrStr` _output ":") _outputstring))
          (bind _outputstring_2 (`self.CombineStringsWithSeparator` (`local.NewGemArray`) ";"))
          (return _outputstring_2)))
      (:`Head`
        (if (`|EnumEquality` (`local.ItemType`) "NewEnumerator1")
          (goto _label)))
      (:`Tail`
        (if (`|EnumEquality` (`local.ItemType`) "NewEnumerator2")
          (goto _label))))))

(fn `Set Weapon Component Mesh`
  (params (WeaponMesh :type "StaticMeshComponent Object Reference") (WeaponData :type "/Game/MultiplayerLobbies/Datatables/ComponentData Structure"))
  (`StaticMeshComponent.SetStaticMesh` WeaponMesh (`.StaticMesh_10_603EC9A743521CB4AF0D318101D7906B` (break `/Game/MultiplayerLobbies/Datatables/BaseItemData` (`.ItemData_2_AB890E3145ADAEB69815B3B9B749E7DE` (break `/Game/MultiplayerLobbies/Datatables/ComponentData` WeaponData))))))