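; Player character that fires staff projectiles and switches to an inventory camera view.
; FireAction plays the staff attack montage; its FireProjectile notify spawns BP_Projectile with info generated from base data and component logics.
; Tick traces from the camera to aim the spawn point at the hit, falling back to a scaled camera-forward vector without camera-location offset.
; ToggleInventoryMode reattaches the camera between the spring arm and a scene component.
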(event `Toggle Inventory Mode`
  (params (Enabled :type Boolean))
  (bind _output_get (set `self.InventoryMode` Enabled))
  (if _output_get
    (`SceneComponent.K2_AttachToComponent` (`self.Camera`) (`self.Scene`) "None" "KeepRelative" "KeepRelative" "KeepRelative" true)
    (else
      (`SceneComponent.K2_AttachToComponent` (`self.Camera`) (`self.SpringArm`) "None" "KeepRelative" "KeepRelative" "KeepRelative" true)))
  (`SceneComponent.K2_SetRelativeLocationAndRotation` :`self` (`self.Camera`)))

(event `self.FireAction`
  (bind _notifyname (`|PlayMontage` (`self.Mesh`) "/Game/Animations/Attack_Staff_Montage.Attack_Staff_Montage")
    (:`OnNotifyBegin`
      (if (== _notifyname "FireProjectile")
        (bind _projectileinfo (`/Game/MultiplayerLobbies/Blueprints/GenericBlueprints.GenerateProjectileInfo` (`self.BaseProjectileInfo`) (`self.ComponentLogics`)))
        (`|SpawnActorFromClass` "/Game/MultiplayerLobbies/Blueprints/BP_Projectile.BP_Projectile_C" (`SceneComponent.K2_GetComponentToWorld` (`self.Projectile Spawn Point`)) "Undefined" "MultiplyWithRoot" null _projectileinfo self)))))

(event `self.ReceiveTick`
  (params (DeltaSeconds :type "Float (single-precision)"))
  (bind _returnvalue (`GameplayStatics.GetPlayerCameraManager` 0))
  (bind _projectile_spawn_point (`self.Projectile Spawn Point`))
  (bind _returnvalue_2 (`SceneComponent.K2_GetComponentLocation` (`self.Projectile Spawn Point`)))
  (bind _returnvalue_3 (`PlayerCameraManager.GetCameraLocation` _returnvalue))
  (bind _returnvalue_4 (* (`KismetMathLibrary.GetForwardVector` (`PlayerCameraManager.GetCameraRotation` _returnvalue)) 10000))
  (`parent.ReceiveTick` DeltaSeconds)
  (bind (_outhit _returnvalue_5) (`KismetSystemLibrary.LineTraceSingle` _returnvalue_3 (+ _returnvalue_3 _returnvalue_4) "TraceTypeQuery1"))
  (if _returnvalue_5
    (`SceneComponent.K2_SetWorldRotation` _projectile_spawn_point (`KismetMathLibrary.FindLookAtRotation` _returnvalue_2 (`.Location` (`GameplayStatics.BreakHitResult` _outhit))) false false)
    (else
      (`SceneComponent.K2_SetWorldRotation` _projectile_spawn_point (`KismetMathLibrary.FindLookAtRotation` _returnvalue_2 _returnvalue_4) false false))))

(fn `UserConstructionScript`
  (`parent.UserConstructionScript`))