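; Actor component that tracks health for its owner and handles healing and incoming damage.
; TakeDamage rejects hits when dead, invincible or blocking, with damage info flags able to bypass invincibility or blocking, and returns whether damage landed.
; Heal and TakeDamage clamp health to the valid range and fire a health-changed dispatcher.
; Other dispatchers report blocks, death, or the damage response for non-lethal hits.
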(fn `Heal`
  (params (Amount :type "Float (double-precision)"))
  (returns (NewHealth :type "Float (double-precision)"))
  (bind _health (`self.Health`))
  (if (not (`self.IsDead`))
    (bind _output_get (set `self.Health` (`KismetMathLibrary.FClamp` (+ Amount _health) 0.0 (`self.MaxHealth`))))
    (`self.OnHealthChanged`)
    (return _output_get)
    (else
      (return _health))))

(fn `Take Damage`
  (params (DamageInfo :type "/Game/MultiplayerLobbies/Blueprints/DamageSystem/DamageInfo Structure"))
  (returns (WasDamaged :type Boolean))
  (bind (_amount _damagetype _damageresponse _shoulddamageinvinvible _canbeblocked) (break `/Game/MultiplayerLobbies/Blueprints/DamageSystem/DamageInfo` DamageInfo))
  (if (`self.IsDead`)
    (return false)
    (elif (and (`self.IsInvincible`) (not _shoulddamageinvinvible))
      (return false)
      (elif (and (`self.IsBlocking`) _canbeblocked)
        (`self.OnBlocked`)
        (return false)
        (else
          (bind _output_get (set `self.Health` (`KismetMathLibrary.FClamp` (- (`self.Health`) _amount) 0.0 (`self.MaxHealth`))))
          (`self.OnHealthChanged`)
          (if (<= _output_get 0.0)
            (set `self.IsDead` true)
            (`self.OnDeath`)
            (else
              (`self.OnDamageResponse` _damageresponse)))
          (return true))))))