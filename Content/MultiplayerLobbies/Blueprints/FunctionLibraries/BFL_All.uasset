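; Blueprint function library for the multiplayer lobby project that handles the player's character choice and audio option saving.
; Character and audio options are written to separate slots, each from a freshly created BP_SV_User save object.
; Loading the character falls back to BP_C_Master when no save exists, without writing that default to disk.
; Separate helpers set and get the current character on the BP_GI_ML game instance.
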(fn `GetCharacterFromGameInstance`
  (returns (Character :type "Character Class Reference"))
  ;[1 1 1] get character from gameinstance
  (bind _asbp_gi_ml (cast `/Game/MultiplayerLobbies/Blueprints/GameInstances/BP_GI_ML` (`GameplayStatics.GetGameInstance` null)))
  (return (`/Game/MultiplayerLobbies/Blueprints/GameInstances/BP_GI_ML.Character` _asbp_gi_ml)))

(fn `GetUserSavedCharacter`
  (returns (Character :type "Character Class Reference"))
  ;[1 1 1] does save game exits
  (bind _returnvalue (`GameplayStatics.DoesSaveGameExist` "Character"))
  (if _returnvalue
    ;[1 1 1] load character from the save
    (bind _returnvalue_2 (`GameplayStatics.LoadGameFromSlot` "Character"))
    (bind _asbp_sv_user (cast `/Game/MultiplayerLobbies/Blueprints/SaveGame/BP_SV_User` _returnvalue_2))
    (return (`/Game/MultiplayerLobbies/Blueprints/SaveGame/BP_SV_User.Character` _asbp_sv_user))
    (else
      ;[1 1 1] create new save for character
      (bind _returnvalue_3 (`GameplayStatics.CreateSaveGameObject` "/Game/MultiplayerLobbies/Blueprints/SaveGame/BP_SV_User.BP_SV_User_C"))
      (bind _output_get (set `/Game/MultiplayerLobbies/Blueprints/SaveGame/BP_SV_User.Character` "/Game/MultiplayerLobbies/Blueprints/Characters/BP_C_Master.BP_C_Master_C" _returnvalue_3))
      (return _output_get))))

(fn `SaveAllAudio`
  (params (S_Options :type "/Game/MultiplayerLobbies/Structures/S_Options Structure"))
  ;[1 1 1] save all audio percentages
  (bind _returnvalue (`GameplayStatics.CreateSaveGameObject` "/Game/MultiplayerLobbies/Blueprints/SaveGame/BP_SV_User.BP_SV_User_C"))
  (set `/Game/MultiplayerLobbies/Blueprints/SaveGame/BP_SV_User.S_Options` S_Options _returnvalue)
  (`GameplayStatics.SaveGameToSlot` _returnvalue "Audio"))

(fn `SaveCharacter`
  (params (Character :type "Character Class Reference"))
  ;[1 1 1] save character to slot
  (bind _returnvalue (`GameplayStatics.CreateSaveGameObject` "/Game/MultiplayerLobbies/Blueprints/SaveGame/BP_SV_User.BP_SV_User_C"))
  (set `/Game/MultiplayerLobbies/Blueprints/SaveGame/BP_SV_User.Character` Character _returnvalue)
  (`GameplayStatics.SaveGameToSlot` _returnvalue "Character"))

(fn `SetCharacterForGameInstance`
  (params (Char :type "Character Class Reference"))
  ;[1 1 1] set character for gameinstance
  (bind _asbp_gi_ml (cast `/Game/MultiplayerLobbies/Blueprints/GameInstances/BP_GI_ML` (`GameplayStatics.GetGameInstance` null)))
  (set `/Game/MultiplayerLobbies/Blueprints/GameInstances/BP_GI_ML.Character` Char _asbp_gi_ml))