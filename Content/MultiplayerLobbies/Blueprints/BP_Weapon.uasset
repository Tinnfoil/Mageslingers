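; BP_Weapon is a weapon actor that ALS characters can pick up and drop.
; Its Construction Script initializes the weapon from its Item data.
; The Pickup and Drop events cast the passed actor to ALS_CharacterBP and have it hold or drop the weapon in hand.
; Pickup also prints the actor's name and reports a failed cast as debug output.
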(event `self.Pickup`
  (params (Actor :type "Actor Object Reference"))
  (`KismetSystemLibrary.PrintString` (`KismetSystemLibrary.GetDisplayName` Actor))
  (bind _asals_character_bp (cast `/ALSV4_CPP/ALV4/Blueprints/CharacterLogic/ALS_CharacterBP` Actor)
    (:`then`
      (`/ALSV4_CPP/ALV4/Blueprints/CharacterLogic/ALS_CharacterBP.HoldItemInHand` _asals_character_bp self))
    (:`CastFailed`
      (`KismetSystemLibrary.PrintString` "Failed Cast"))))

(event `self.Drop`
  (params (Actor :type "Actor Object Reference"))
  (bind _asals_character_bp (cast `/ALSV4_CPP/ALV4/Blueprints/CharacterLogic/ALS_CharacterBP` Actor))
  (`/ALSV4_CPP/ALV4/Blueprints/CharacterLogic/ALS_CharacterBP.DropItemInHand` _asals_character_bp self))

(fn `UserConstructionScript`
  (`/Game/MultiplayerLobbies/Datatables/GenericBlueprints.Initialize Weapon Component` self (`self.Item`)))