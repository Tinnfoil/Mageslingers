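; Lobby game mode for multiplayer that tracks joined BP_PC_Lobby controllers and runs kicking, map selection and match start on the server.
; Joins and logouts update the controller array and rebuild every client's player list through client calls; logout also frees the start point and destroys the character.
; The current map, defaulting from the D_Maps table, is pushed to all HUDs.
; Starting shows loading screens, then server-travels to that map.
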(event `Server_KickPlayerFromTheLobby`
  (params (PlayerLobbyIndex :type Integer))
  ;[1 1 1] kick player from the lobby on server
  (`/Game/MultiplayerLobbies/Blueprints/Controllers/BP_PC_Lobby.Client_KickPlayerFromTheLobby` (`|GetArrayItem` (`self.AllLobbyPlayers`) PlayerLobbyIndex)))

(event `self.HandleStartingNewPlayer`
  (params (NewPlayer :type "PlayerController Object Reference"))
  ;[1 1 1] create lobby widget, spawn characters and update lobby infromation to players
  (bind _asbp_pc_lobby (cast `/Game/MultiplayerLobbies/Blueprints/Controllers/BP_PC_Lobby` NewPlayer))
  (`KismetArrayLibrary.Array_Add` (`self.AllLobbyPlayers`) _asbp_pc_lobby)
  (`/Game/MultiplayerLobbies/Blueprints/Controllers/BP_PC_Lobby.Client_CreateHUDAndSpawnCharacter` _asbp_pc_lobby)
  (`self.UpdateMapInfoForAllClients` (`self.CurrentMap`))
  (`self.Server_UpdateLobbyPlayerlist`))

(event `Server_StartGame`
  ;[1 1 1] start match and server travel into level
  (`self.ServerTravelIntoLevel`))

(event `Server_UpdateServerInfoOnClients`
  (params (S_Maps :type "/Game/MultiplayerLobbies/Structures/S_Maps Structure"))
  ;[1 1 1] update map information to all players
  (bind _output_get (set `self.CurrentMap` S_Maps))
  (for _array_element (`self.AllLobbyPlayers`)
    (`/Game/MultiplayerLobbies/Blueprints/Controllers/BP_PC_Lobby.Client_UpdateMapInfoOnHUD` _array_element _output_get)))

(event `Server_UpdateLobbyPlayerlist`
  ;[1 1 1] update playerlist information on server
  (`self.UpdatePlayerlistInformation`))

(event `self.K2_OnLogout`
  (params (ExitingController :type "Controller Object Reference"))
  ;[1 1 1] logout player when kicked or disconnected
  (`self.LogoutUserWhenDisconnecting` ExitingController))

(fn `LogoutUserWhenDisconnecting`
  (params (InputPin :type "Controller Object Reference"))
  ;[1 1 1] logout user, remove player from "AllLobbyPlayers", update playerlist on server
  (for (_array_element _array_index) (`self.AllLobbyPlayers`)
    (if (== _array_element InputPin)
      (break)))
  (set `PlayerStart.PlayerStartTag` "None" (`/Game/MultiplayerLobbies/Blueprints/Controllers/BP_PC_Lobby.LobbyPlayerStart` _array_element))
  (`self.K2_DestroyActor` (`/Game/MultiplayerLobbies/Blueprints/Controllers/BP_PC_Lobby.LobbyCharacter` _array_element))
  (`KismetArrayLibrary.Array_Remove` (`self.AllLobbyPlayers`) _array_index)
  (`self.Server_UpdateLobbyPlayerlist`))

(fn `ServerTravelIntoLevel`
  ;[1 1 1] show loading screens for the players and server travel into level
  (for _array_element (`self.AllLobbyPlayers`)
    (`/Game/MultiplayerLobbies/Blueprints/Controllers/BP_PC_Lobby.Client_CreateLoadingScreen` _array_element))
  (`AdvancedSessionsLibrary.ServerTravel` (`KismetStringLibrary.Concat_StrStr` "/Game/MultiplayerLobbies/Maps/" (`.MapServerTravel_10_ABE1869A49AC3B78614CF6BBD72FF46E` (break `/Game/MultiplayerLobbies/Structures/S_Maps` (`self.CurrentMap`)))) (and (`KismetSystemLibrary.IsStandalone`) (`self.bUseSeamlessTravel`))))

(fn `UpdateMapInfoForAllClients`
  (params (CurrentMap :type "/Game/MultiplayerLobbies/Structures/S_Maps Structure"))
  ;[1 1 1] get default map from datatable and update it for all clients
  (if (`KismetStringLibrary.EqualEqual_StrStr` (`.MapName_12_78E99B0D4B5170E0248315940147EEE6` (break `/Game/MultiplayerLobbies/Structures/S_Maps` (`self.CurrentMap`))))
    (bind _returnvalue (`|GetDataTableRow` "/Game/MultiplayerLobbies/Datatables/D_Maps.D_Maps" "Default")
      (:`then`
        (bind _output_get (set `self.CurrentMap` _returnvalue))
        (`self.Server_UpdateServerInfoOnClients` _output_get)))
    (else
      (bind _output_get_2 (set `self.CurrentMap` CurrentMap))
      (`self.Server_UpdateServerInfoOnClients` _output_get_2))))

(fn `UpdatePlayerlistInformation`
  (bind _alllobbyplayers (`self.AllLobbyPlayers`))
  ;[1 1 1] clear all players from the list, update list with new players
  (for _array_element _alllobbyplayers
    (`/Game/MultiplayerLobbies/Blueprints/Controllers/BP_PC_Lobby.Client_ClearAllPlayersFromTheList` _array_element)
    (for (_array_element_2 _array_index) _alllobbyplayers
      (`/Game/MultiplayerLobbies/Blueprints/Controllers/BP_PC_Lobby.Client_AddNewPlayerToList` _array_element (`PlayerState.GetPlayerName` (`Controller.PlayerState` _array_element_2)) _array_index))))

(fn `UserConstructionScript`)