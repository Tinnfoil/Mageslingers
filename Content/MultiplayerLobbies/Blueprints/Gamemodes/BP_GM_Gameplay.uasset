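; Gameplay game mode for the multiplayer lobby system that tracks connected players and returns them to the Lobby map.
; PostLogin adds each ALS_Player_Controller to AllGameplayPlayers.
; ReturnToLobby has each tracked controller create a client loading screen, then calls ServerTravel to the Lobby map, feeding UseSeamlessTravel into its Absolute input.
; An older console-command servertravel is left unconnected.
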(event `self.HandleStartingNewPlayer`
  (params (NewPlayer :type "PlayerController Object Reference"))
  ;[1 1 1] add new player to "AllGameplayPlayers"
)

(event `self.K2_PostLogin`
  (params (NewPlayer :type "PlayerController Object Reference"))
  ;[1 1 1] add new player to "AllGameplayPlayers"
  (bind _asals_player_controller (cast `/ALSV4_CPP/ALV4/Blueprints/CharacterLogic/ALS_Player_Controller` NewPlayer))
  (`KismetArrayLibrary.Array_Add` (`self.AllGameplayPlayers`) _asals_player_controller))

(fn `Return to Lobby`
  ;[1 1 1] show loading screens for the players and server travel into level
  (for _array_element (`self.AllGameplayPlayers`)
    (`/ALSV4_CPP/ALV4/Blueprints/CharacterLogic/ALS_Player_Controller.Client_CreateLoadingScreen` _array_element))
  (`AdvancedSessionsLibrary.ServerTravel` (`KismetStringLibrary.Concat_StrStr` "/Game/MultiplayerLobbies/Maps/" "Lobby") (`self.bUseSeamlessTravel`)))

(fn `UserConstructionScript`)