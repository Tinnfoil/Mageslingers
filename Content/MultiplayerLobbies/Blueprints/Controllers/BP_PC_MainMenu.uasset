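; Main menu player controller that sets up the menu screen and preview character for a multiplayer lobby game.
; BeginPlay destroys any existing session, then adds input contexts, creates the menu widget with UI-only input and spawns the user's saved character.
; The spawn event replaces any previous character at the first PlayerStart, then saves it and stores it in the GameInstance.
; The view switches to the first BP_C_Main actor.
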(event `self.ReceiveBeginPlay`
  (bind _returnvalue (pcsubsystem `EnhancedInputLocalPlayerSubsystem` (`GameplayStatics.GetPlayerController` 0)))
  ;[1 1 1] Create HUD, spawn main menu character and add input mapping contexts
  (`DestroySessionCallbackProxy.DestroySession` self
    (:`then`
      (`EnhancedInputSubsystemInterface.AddMappingContext` _returnvalue "/Game/MultiplayerLobbies/Input/InputMappingContexts/IMC_Actions.IMC_Actions" 0 (struct))
      (`EnhancedInputSubsystemInterface.AddMappingContext` _returnvalue "/Game/MultiplayerLobbies/Input/InputMappingContexts/IMC_Movement.IMC_Movement" 0 (struct))
      (`self.Client_CreateMainMenuWidget`)
      (`self.Client_SpawnMainMenuCharacter` (`/Game/MultiplayerLobbies/Blueprints/FunctionLibraries/BFL_All.GetUserSavedCharacter`))
      (`self.Client_SetNewViewTarget`))))

(event `Client_SpawnMainMenuCharacter`
  (params (SpawnedCharacter :type "Character Class Reference"))
  ;[1 1 1] spawn main menu character
  (bind _spawnedcharacter (`self.SpawnedCharacter`)
    (:`then`
      (`self.K2_DestroyActor` _spawnedcharacter))
    (:`else`
      _))
  (bind _outactors (`GameplayStatics.GetAllActorsOfClass` "/Script/Engine.PlayerStart"))
  (bind _returnvalue (`|SpawnActorFromClass` SpawnedCharacter (`self.GetTransform` (`|GetArrayItem` _outactors)) "Undefined" "SelectDefaultAtRuntime" null null))
  (set `self.SpawnedCharacter` _returnvalue)
  (`/Game/MultiplayerLobbies/Blueprints/FunctionLibraries/BFL_All.SaveCharacter` SpawnedCharacter)
  (`/Game/MultiplayerLobbies/Blueprints/FunctionLibraries/BFL_All.SetCharacterForGameInstance` SpawnedCharacter))

(event `Client_SetNewViewTarget`
  ;[1 1 1] set new view target for client
  (bind _outactors (`GameplayStatics.GetAllActorsOfClass` "/Game/MultiplayerLobbies/Blueprints/Cameras/BP_C_Main.BP_C_Main_C"))
  (`self.SetViewTargetWithBlend` (`|GetArrayItem` _outactors)))

(event `Client_CreateMainMenuWidget`
  ;[1 1 1] create main menu widget on client
  (bind _returnvalue (`|CreateWidget` "/Game/MultiplayerLobbies/Widgets/WBP_MainMenu.WBP_MainMenu_C"))
  (`UserWidget.AddToViewport` _returnvalue 0)
  (`WidgetBlueprintLibrary.SetInputMode_UIOnlyEx` (`GameplayStatics.GetPlayerController` 0) _returnvalue))

(fn `UserConstructionScript`)