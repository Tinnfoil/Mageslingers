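; Gameplay player controller for a multiplayer game that spawns the player's chosen character and opens the in-game menu.
; On BeginPlay it adds Enhanced Input contexts, then a client RPC clears widgets and passes the GameInstance's character class to a server RPC.
; The server claims a free PlayerStart by tagging it "Reserved", then spawns and possesses the character there.
; The menu action switches to UI-only input and halts the character.
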(event `self.ReceiveBeginPlay`
  (bind _returnvalue (pcsubsystem `EnhancedInputLocalPlayerSubsystem` (`GameplayStatics.GetPlayerController` 0)))
  ;[1 1 1] BeginPlay, add mapping contexts and spawn character
  (`EnhancedInputSubsystemInterface.AddMappingContext` _returnvalue "/Game/MultiplayerLobbies/Input/InputMappingContexts/IMC_Actions.IMC_Actions" 0 (struct))
  (`EnhancedInputSubsystemInterface.AddMappingContext` _returnvalue "/Game/MultiplayerLobbies/Input/InputMappingContexts/IMC_Movement.IMC_Movement" 0 (struct))
  (`self.Client_SpawnCharacterOnClient`))

(event `Server_SpawnCharacterOnServer`
  (params (Character :type "Character Class Reference"))
  ;[1 1 1] spawn character on server
  (`self.SpawnCharacter` Character))

(event `Client_SpawnCharacterOnClient`
  ;[1 1 1] spawn character on client
  (`WidgetLayoutLibrary.RemoveAllWidgets`)
  (`self.Server_SpawnCharacterOnServer` (`/Game/MultiplayerLobbies/Blueprints/FunctionLibraries/BFL_All.GetCharacterFromGameInstance`))
  (`WidgetBlueprintLibrary.SetInputMode_GameOnly` self))

(event `EnhancedInput|/Game/MultiplayerLobbies/Input/InputActions/AI_InGameMenu`
  (params (ActionValue :type Boolean) (ElapsedSeconds :type "Float (double-precision)") (TriggeredSeconds :type "Float (double-precision)") (InputAction :type "InputAction Object Reference" :default "/Game/MultiplayerLobbies/Input/InputActions/AI_InGameMenu.AI_InGameMenu"))
  ;[1 1 1] create in game menu
  (:`Triggered`
    (`self.CreateInGameMenu`)))

(fn `CreateInGameMenu`
  (bind _returnvalue (`GameplayStatics.GetPlayerCharacter` 0))
  ;[1 1 1] create in game menu, show mouse cursor and stop character movement
  (bind _returnvalue_2 (`|CreateWidget` "/Game/MultiplayerLobbies/Widgets/WBP_InGameMenu.WBP_InGameMenu_C"))
  (`UserWidget.AddToViewport` _returnvalue_2 0)
  (set `self.bShowMouseCursor` true)
  (`WidgetBlueprintLibrary.SetInputMode_UIOnlyEx` self _returnvalue_2)
  (`MovementComponent.StopMovementImmediately` (`Pawn.GetMovementComponent` _returnvalue))
  (`self.DisableInput` _returnvalue self))

(fn `SpawnCharacter`
  (params (Character :type "Character Class Reference"))
  ;[1 1 1] spawn actor and find free playerstart
  (bind _outactors (`GameplayStatics.GetAllActorsOfClass` "/Script/Engine.PlayerStart"))
  (for _array_element _outactors
    (if (!= (`PlayerStart.PlayerStartTag` _array_element) "Reserved")
      (set `PlayerStart.PlayerStartTag` "Reserved" _array_element)
      (break)))
  (bind _returnvalue (`|SpawnActorFromClass` Character (`self.GetTransform` _array_element) "Undefined" "SelectDefaultAtRuntime" null null))
  (`self.Possess` _returnvalue))

(fn `UserConstructionScript`)