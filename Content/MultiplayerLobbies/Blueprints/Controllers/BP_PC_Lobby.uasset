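; Lobby player controller that gives each player a lobby HUD, a preview character and a shared camera view.
; BeginPlay adds input mappings and blends the view to the main camera actor.
; Client events drive the player list, map info, loading screen and kick-to-main-menu with session destruction.
; The saved character choice goes to a server event, which spawns it at the first free PlayerStart, tagging that start "Reserved".
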(event `self.ReceiveBeginPlay`
  (bind _returnvalue (pcsubsystem `EnhancedInputLocalPlayerSubsystem` (`GameplayStatics.GetPlayerController` 0)))
  ;[1 1 1] Beginplay, add mapping contexts and set new view target
  (`EnhancedInputSubsystemInterface.AddMappingContext` _returnvalue "/Game/MultiplayerLobbies/Input/InputMappingContexts/IMC_Actions.IMC_Actions" 0 (struct))
  (`EnhancedInputSubsystemInterface.AddMappingContext` _returnvalue "/Game/MultiplayerLobbies/Input/InputMappingContexts/IMC_Movement.IMC_Movement" 0 (struct))
  (`self.Client_SetNewViewTarget`))

(event `Client_SpawnCharacterForLobby`
  ;[1 1 1] spawn character for lobby on client
  (`self.Server_SpawnCharacterForLobby` (`/Game/MultiplayerLobbies/Blueprints/FunctionLibraries/BFL_All.GetUserSavedCharacter`)))

(event `Client_AddNewPlayerToList`
  (params (LobbyPlayerName :type String) (LobbyPlayerIndex :type Integer))
  ;[1 1 1] playerlist actions on client
  ;;[1 1 1] add new players to list
  (`/Game/MultiplayerLobbies/Widgets/WBP_Lobby.AddNewPlayersToList` (`self.WBP_Lobby`) LobbyPlayerName LobbyPlayerIndex))

(event `Client_CreateHUDAndSpawnCharacter`
  ;[1 1 1] create lobby on client
  (bind _returnvalue (`|CreateWidget` "/Game/MultiplayerLobbies/Widgets/WBP_Lobby.WBP_Lobby_C"))
  (bind _output_get (set `self.WBP_Lobby` _returnvalue))
  (`UserWidget.AddToViewport` _output_get 0)
  (`WidgetBlueprintLibrary.SetInputMode_UIOnlyEx` (`GameplayStatics.GetPlayerController` 0) _output_get)
  (`self.Client_SpawnCharacterForLobby`))

(event `Client_ClearAllPlayersFromTheList`
  ;[1 1 1] playerlist actions on client
  ;;[1 1 1] clear players from the list
  (`/Game/MultiplayerLobbies/Widgets/WBP_Lobby.ClearPlayersFromList` (`self.WBP_Lobby`)))

(event `Server_SpawnCharacterForLobby`
  (params (Character :type "Character Class Reference"))
  ;[1 1 1] spawn character and find free playerstart on server
  (bind _outactors (`GameplayStatics.GetAllActorsOfClass` "/Script/Engine.PlayerStart"))
  (for _array_element _outactors
    (if (!= (`PlayerStart.PlayerStartTag` _array_element) "Reserved")
      (bind _output_get (set `self.LobbyPlayerStart` _array_element))
      (set `PlayerStart.PlayerStartTag` "Reserved" _output_get)
      (break)))
  (bind _returnvalue (`|SpawnActorFromClass` Character (`self.GetTransform` _array_element) "Undefined" "SelectDefaultAtRuntime" null null))
  (set `self.LobbyCharacter` _returnvalue))

(event `Client_SetNewViewTarget`
  ;[1 1 1] set new view target to main camera
  (bind _outactors (`GameplayStatics.GetAllActorsOfClass` "/Game/MultiplayerLobbies/Blueprints/Cameras/BP_C_Main.BP_C_Main_C"))
  (`self.SetViewTargetWithBlend` (`|GetArrayItem` _outactors)))

(event `Client_CreateLoadingScreen`
  ;[1 1 1] create loading screen on client
  (bind _returnvalue (`|CreateWidget` "/Game/MultiplayerLobbies/Widgets/WBP_LoadingScreen.WBP_LoadingScreen_C"))
  (`UserWidget.AddToViewport` _returnvalue 0))

(event `Client_UpdateMapInfoOnHUD`
  (params (S_Maps :type "/Game/MultiplayerLobbies/Structures/S_Maps Structure"))
  ;[1 1 1] update map info on client
  (`/Game/MultiplayerLobbies/Widgets/WBP_Lobby.UpdateMapInfo` (`self.WBP_Lobby`) S_Maps))

(event `Client_KickPlayerFromTheLobby`
  ;[1 1 1] kick player from the lobby
  (`DestroySessionCallbackProxy.DestroySession` self
    (:`then`
      (`GameplayStatics.OpenLevel` "MainMenu"))))

(fn `LoadCharacterFromSave`
  (returns (Character :type "Character Class Reference"))
  ;[1 1 1] get user character
  (return (`/Game/MultiplayerLobbies/Blueprints/FunctionLibraries/BFL_All.GetUserSavedCharacter`)))

(fn `UserConstructionScript`)