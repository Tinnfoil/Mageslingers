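; Weapon actor for a multiplayer game that an ALS character can pick up to hold in hand and drop.
; Pickup and Drop cast the passed actor to ALS_CharacterBP and call its hold or drop item functions.
; The construction script calls ConstructWeapon with the Item data, and the RepNotify on Item builds the weapon mesh on BaseMesh from that data.
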(event `Event Pickup`
  (params (Actor :type "Actor Object Reference"))
  (`KismetSystemLibrary.PrintString` (`KismetSystemLibrary.GetDisplayName` Actor))
  (bind _asals_character_bp (cast `/ALSV4_CPP/ALV4/Blueprints/CharacterLogic/ALS_CharacterBP` Actor)
    (:`then`
      (`/ALSV4_CPP/ALV4/Blueprints/CharacterLogic/ALS_CharacterBP.HoldItemInHand` :`self` _asals_character_bp :`ItemToHold` self))
    (:`CastFailed`
      (`KismetSystemLibrary.PrintString` "Failed Cast"))))

(event `Event Drop`
  (params (Actor :type "Actor Object Reference"))
  (bind _asals_character_bp (cast `/ALSV4_CPP/ALV4/Blueprints/CharacterLogic/ALS_CharacterBP` Actor))
  (`/ALSV4_CPP/ALV4/Blueprints/CharacterLogic/ALS_CharacterBP.DropItemInHand` _asals_character_bp))

(event `Construct_Weapon`
  (params (`Weapon Data` :type "/Game/MultiplayerLobbies/Datatables/WeaponItemData Structure"))
  (set `self.Item` `Weapon Data`))

(fn `OnRep_Item`
  (`/Game/MultiplayerLobbies/Datatables/GenericBlueprints.Construct Weapon Mesh` (`self.BaseMesh`) (`self.Item`) self))

(fn `UserConstructionScript`
  (`self.Construct_Weapon` self (`self.Item`)))