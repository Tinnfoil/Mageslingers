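; Actor component that holds a BaseCharacter_BP's inventory and handles slot swaps, including fitting pieces and gems into the held weapon.
; BeginPlay pads Items to the slot limit; adding fills the first "Null"-named slot.
; SwapInventorySlots calls ValidInsert in both directions, which writes as it validates, so a failed second insert is not rolled back.
; ValidInsert checks piece type or gem database compatibility, then rebuilds HeldItemData or overwrites the item slot.
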(event `self.ReceiveBeginPlay`
  (bind _asbase_character_bp (cast `/Game/MultiplayerLobbies/Blueprints/BaseCharacter_BP` (`self.GetOwner`)))
  (set `self.OwningCharacter` _asbase_character_bp)
  (while (< (`KismetArrayLibrary.Array_Length` (`self.Items`)) (`self.MaxInventorySlots`))
    (`KismetArrayLibrary.Array_Add` (`self.Items`) (make `/Game/MultiplayerLobbies/Datatables/BaseItemData` "Null" null null "NewEnumerator4" "/Game/MultiplayerLobbies/Blueprints/BP_InteractableObject.BP_InteractableObject_C" "/Game/MultiplayerLobbies/Blueprints/WeaponComponents/ComponentLogic.ComponentLogic_C"))))

(event `Spawn_TestItems`)

(fn `AddItemToInventory`
  (params (ItemData :type "/Game/MultiplayerLobbies/Datatables/BaseItemData Structure (by ref)"))
  (for (_array_element _array_index) (`self.Items`)
    (if (== (`.Name_11_B8DF43004E223A93E21556A5E1CBF881` (break `/Game/MultiplayerLobbies/Datatables/BaseItemData` _array_element)) "Null")
      (`KismetArrayLibrary.Array_Set` (`self.Items`) _array_index ItemData)
      (break))))

(fn `SwapInventorySlots`
  (params (SlotIndex1 :type Integer) (InsertType1 :type "/Game/MultiplayerLobbies/Datatables/InventoryInsertType Enum" :default "NewEnumerator0") (OwningType1 :type "/Game/MultiplayerLobbies/Datatables/WeaponComponentType Enum" :default "NewEnumerator4") (ItemData1 :type "/Game/MultiplayerLobbies/Datatables/BaseItemData Structure") (SlotIndex2 :type Integer) (InsertType2 :type "/Game/MultiplayerLobbies/Datatables/InventoryInsertType Enum" :default "NewEnumerator0") (OwningType2 :type "/Game/MultiplayerLobbies/Datatables/WeaponComponentType Enum" :default "NewEnumerator4") (ItemData2 :type "/Game/MultiplayerLobbies/Datatables/BaseItemData Structure"))
  (returns (SwapSuccessful :type Boolean))
  (locals (CachedItemData :type "/Game/MultiplayerLobbies/Datatables/BaseItemData Structure") (InsertingData :type "/Game/MultiplayerLobbies/Datatables/BaseItemData Structure") (InsertType :type "/Game/MultiplayerLobbies/Datatables/WeaponComponentType Enum"))
  (bind _output_get (set `local.InsertingData` ItemData1))
  (bind _output_get_2 (set `local.CachedItemData` ItemData2))
  (bind _isvalid (`self.ValidInsert` _output_get SlotIndex2 InsertType2 OwningType2))
  (if _isvalid
    (bind _isvalid_2 (`self.ValidInsert` _output_get_2 SlotIndex1 InsertType1 OwningType1))
    (if _isvalid_2
      (return true)
      (else
        (return false)))
    (else
      (`KismetSystemLibrary.PrintString` "Cannot Swap")
      (return false))))

(fn `ValidInsert`
  (params (InsertingData :type "/Game/MultiplayerLobbies/Datatables/BaseItemData Structure") (Index :type Integer) (InsertType :type "/Game/MultiplayerLobbies/Datatables/InventoryInsertType Enum" :default "NewEnumerator0") (OwningType :type "/Game/MultiplayerLobbies/Datatables/WeaponComponentType Enum" :default "NewEnumerator4"))
  (returns (IsValid :type Boolean))
  (locals (TempInsertType :type "/Game/MultiplayerLobbies/Datatables/WeaponComponentType Enum") (ReturnBool :type Boolean) (HeadPieceData :type "/Game/MultiplayerLobbies/Datatables/ComponentData Structure") (BodyPieceData :type "/Game/MultiplayerLobbies/Datatables/ComponentData Structure") (TailPieceData :type "/Game/MultiplayerLobbies/Datatables/ComponentData Structure") (GemData :type String) (LocalIndex :type Integer) (LocalInsertingData :type "/Game/MultiplayerLobbies/Datatables/BaseItemData Structure") (TempOwningType :type "/Game/MultiplayerLobbies/Datatables/WeaponComponentType Enum") (NewLocalVar :type "/Game/MultiplayerLobbies/Datatables/InventoryInsertType Enum" :default "NewEnumerator0"))
  (bind (_name _staticmesh _icon _type) (break `/Game/MultiplayerLobbies/Datatables/BaseItemData` InsertingData))
  (bind _insertingdata (`local.InsertingData`))
  (bind _componentdata (make `/Game/MultiplayerLobbies/Datatables/ComponentData` _insertingdata))
  (bind (_headpiece _mainbody _tailpiece _gems) (break `/Game/MultiplayerLobbies/Datatables/WeaponItemData` (`/Game/MultiplayerLobbies/Blueprints/BaseCharacter_BP.HeldItemData` (`self.OwningCharacter`))))
  (set `local.LocalInsertingData` InsertingData)
  (set `local.LocalIndex` Index)
  (set `local.TempOwningType` OwningType)
  (switch `/Game/MultiplayerLobbies/Datatables/InventoryInsertType` InsertType
    (:`NewEnumerator0`
      (set `local.TempInsertType` "NewEnumerator0")
      (bind _output_get (set `local.ReturnBool` (and (or (`/Game/MultiplayerLobbies/Blueprints/BaseCharacter_BP.IsHoldingItem` (`self.OwningCharacter`)) (`|EnumEquality` (`local.TempInsertType`) "NewEnumerator0")) (or (`|EnumEquality` _type "NewEnumerator4") (`|EnumEquality` _type (`local.TempInsertType`)))) :!label _label))
      (if _output_get
        (set `local.BodyPieceData` _mainbody :!label _label_2)
        (set `local.HeadPieceData` _headpiece)
        (set `local.TailPieceData` _tailpiece)
        (bind _output_get_2 (set `local.GemData` _gems))
        (switch `/Game/MultiplayerLobbies/Datatables/WeaponComponentType` (`local.TempInsertType`)
          (:`NewEnumerator0`
            (set `local.BodyPieceData` _componentdata))
          (:`NewEnumerator1`
            (set `local.HeadPieceData` _componentdata))
          (:`NewEnumerator2`
            (set `local.TailPieceData` _componentdata))
          (:`NewEnumerator3`
            (bind _gemdata (`/Game/MultiplayerLobbies/Blueprints/GenericBlueprints.Set Gems For Component` (`local.TempOwningType`) _output_get_2 (`local.LocalIndex`) (`.Name_11_B8DF43004E223A93E21556A5E1CBF881` (break `/Game/MultiplayerLobbies/Datatables/BaseItemData` _insertingdata))))
            (`KismetSystemLibrary.PrintString` "Success")
            (set `local.GemData` _gemdata)))
        (set `/Game/MultiplayerLobbies/Blueprints/BaseCharacter_BP.HeldItemData` (make `/Game/MultiplayerLobbies/Datatables/WeaponItemData` (`local.HeadPieceData`) (`local.BodyPieceData`) (`local.TailPieceData`) (`local.GemData`)) (`self.OwningCharacter`))
        (return (`local.ReturnBool`))
        (else
          _)))
    (:`NewEnumerator1`
      (set `local.TempInsertType` "NewEnumerator1")
      (goto _label))
    (:`NewEnumerator2`
      (set `local.TempInsertType` "NewEnumerator2")
      (goto _label))
    (:`NewEnumerator3`
      (set `local.TempInsertType` "NewEnumerator3")
      (bind _returnvalue (`|GetDataTableRow` "/Game/MultiplayerLobbies/Datatables/DB_GemDatabase.DB_GemDatabase" (`KismetStringLibrary.Conv_StringToName` _name))
        (:`then`
          (bind (_itemdata _validpiecetype) (break `/Game/MultiplayerLobbies/Datatables/GemData` _returnvalue))
          (bind _output_get_3 (set `local.ReturnBool` (and (or (`|EnumEquality` _type "NewEnumerator4") (`|EnumEquality` _type "NewEnumerator3")) (or (`|EnumEquality` _validpiecetype (`local.TempOwningType`)) (`|EnumEquality` _validpiecetype "NewEnumerator4")))))
          (if _output_get_3
            (goto _label_2)
            (else
              _)))
        (:`RowNotFound`
          _))
      (`KismetSystemLibrary.PrintString` "Invalid Gem Insert")
      (return false))
    (:`NewEnumerator4`
      (bind _output_get_4 (set `local.ReturnBool` true))
      (if _output_get_4
        (for (_ _array_index) (`self.Items`)
          (if (== _array_index (`local.LocalIndex`))
            (`KismetArrayLibrary.Array_Set` (`self.Items`) _array_index (`local.LocalInsertingData`))
            (break)))
        (return (`local.ReturnBool`))
        (else
          (return false)))))
  (`KismetSystemLibrary.PrintString` "NEED COMPONENT")
  (return false))