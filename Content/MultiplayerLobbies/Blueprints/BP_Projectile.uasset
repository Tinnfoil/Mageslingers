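; Projectile actor that damages characters it hits, configured by a ProjectileInfo struct.
; The construction script feeds that struct into ProjectileMovement for initial speed, homing and whether it bounces, without applying the bounce count or a homing target.
; A BaseMesh hit passes the damage info to any BaseCharacter_BP.
; If DestroyOnHit is set, it then spawns the destroy effect aligned to the surface normal and destroys itself.
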(event `self.BaseMesh.OnComponentHit`
  (params (HitComponent :type "PrimitiveComponent Object Reference") (OtherActor :type "Actor Object Reference") (OtherComp :type "PrimitiveComponent Object Reference") (NormalImpulse :type "Vector Structure") (Hit :type "HitResult Structure (by ref)"))
  (bind (_bblockinghit _binitialoverlap _time _distance _location _impactpoint _normal) (`GameplayStatics.BreakHitResult` Hit))
  (bind _asbase_character_bp (cast `/ALSV4_CPP/ALV4/Blueprints/CharacterLogic/BaseCharacter_BP` OtherActor)
    (:`then`
      (`/ALSV4_CPP/ALV4/Blueprints/CharacterLogic/BaseCharacter_BP.TakeDamage` _asbase_character_bp (`.DamageInfo_3_8082F53F46558311B8C86CBF3F6EFCFF` (break `/Game/MultiplayerLobbies/Blueprints/DamageSystem/ProjectileInfo` (`self.ProjectileInfo`)))))
    (:`CastFailed`
      _))
  (if (`self.DestroyOnHit`)
    (bind _returnvalue (`|SpawnActorFromClass` "/Game/Effects/ProjectileDestroyEffect.ProjectileDestroyEffect_C" (`KismetMathLibrary.Conv_VectorToTransform` _location) "AlwaysSpawn" "MultiplyWithRoot" null null))
    (`self.K2_SetActorRotation` _returnvalue (`KismetMathLibrary.MakeRotFromZX` _normal (`SceneComponent.GetForwardVector` (`BaseObject.BaseMesh` _returnvalue))) false)
    (`self.K2_DestroyActor`)))

(fn `UserConstructionScript`
  (bind _projectilemovement (`self.ProjectileMovement`))
  (bind (_damageinfo _speed _bounces _homing) (break `/Game/MultiplayerLobbies/Blueprints/DamageSystem/ProjectileInfo` (`self.ProjectileInfo`)))
  (set `ProjectileMovementComponent.InitialSpeed` _speed _projectilemovement)
  (if (> _bounces 0)
    (set `ProjectileMovementComponent.bShouldBounce` true _projectilemovement)
    (else
      (set `ProjectileMovementComponent.bShouldBounce` false _projectilemovement)))
  (set `ProjectileMovementComponent.bIsHomingProjectile` _homing (`self.ProjectileMovement`)))