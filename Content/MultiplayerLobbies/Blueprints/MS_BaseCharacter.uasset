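; Base multiplayer character that carries modular weapons in hand and on its back, with an inventory and health.
; RepNotify weapon data rebuilds each socket-aligned mesh and stores gem data, with the held weapon also rebuilding its component logic.
; Weapons can be swapped or dropped as physics-simulated BP_Weapon actors.
; BPCDamageSystem handles health calls and triggers ragdoll on death, after which a Tick countdown heals and revives the character.
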(event `self.ReceiveTick`
  (params (DeltaSeconds :type "Float (single-precision)"))
  (bind _bpc_damagesystem (`self.BPC_DamageSystem`))
  (if (`/Game/MultiplayerLobbies/Blueprints/DamageSystem/BPC_DamageSystem.IsDead` (`self.BPC_DamageSystem`))
    (bind _output_get (set `self.GetUpTime` (- (`self.GetUpTime`) DeltaSeconds)))
    (if (< _output_get 0.0)
      (set `/Game/MultiplayerLobbies/Blueprints/DamageSystem/BPC_DamageSystem.IsDead` false _bpc_damagesystem)
      (`/Game/MultiplayerLobbies/Blueprints/DamageSystem/BPC_DamageSystem.Heal` _bpc_damagesystem 100.0)
      (`self.RagdollEnd`)
      (set `self.GetUpTime` 2.0))))

(event `SwapWeapons`
  (bind _output_get (set `self.TempWeaponData` (`self.HeldItemData`)))
  (set `self.HeldItemData` (`self.HeldBackItemData`))
  (set `self.HeldBackItemData` _output_get))

(event `Pickup Item`
  (params (`Item Data` :type "/Game/MultiplayerLobbies/Datatables/BaseItemData Structure"))
  (`/Game/MultiplayerLobbies/Blueprints/InventoryComponent.AddItemToInventory` (`self.InventoryComponent`) `Item Data`))

(event `UpdateHeldItem`
  (params (HeldItemData :type "/Game/MultiplayerLobbies/Datatables/WeaponItemData Structure"))
  (set `self.HeldItemData` HeldItemData))

(event `UpdateBackHeldItem`
  (params (HeldBackItemData :type "/Game/MultiplayerLobbies/Datatables/WeaponItemData Structure"))
  (set `self.HeldBackItemData` HeldBackItemData))

(event `self.HeldItemMesh.OnBeginCursorOver`
  (params (TouchedComponent :type "PrimitiveComponent Object Reference"))
  (`KismetSystemLibrary.PrintString` (`KismetSystemLibrary.GetDisplayName` TouchedComponent)))

(event `TestEvent`
  (bind _items (`/Game/MultiplayerLobbies/Blueprints/InventoryComponent.Items` (`self.InventoryComponent`)))
  (`/Game/MultiplayerLobbies/Blueprints/InventoryComponent.Spawn_TestItems` (`self.InventoryComponent`))
  (for _array_element _items
    (`|SpawnActorFromClass` "/Game/MultiplayerLobbies/Blueprints/BP_PickupableObject.BP_PickupableObject_C" (`self.GetTransform`) "Undefined" "MultiplyWithRoot" null _array_element null))
  (`KismetArrayLibrary.Array_Clear` _items))

(event `Death`
  (`self.RagdollAction`)
  (set `self.GetUpTime` 2.0))

(event `DamageResponse`
  (params (Response :type "/Game/MultiplayerLobbies/Blueprints/DamageSystem/DamageResponse Enum" :default "NewEnumerator2")))

(fn `DropItemInHand`
  (bind _returnvalue (`|SpawnActorFromClass` "/Game/MultiplayerLobbies/Blueprints/BP_Weapon.BP_Weapon_C" (`SceneComponent.GetSocketTransform` (`self.TargetSkeletalMesh`) "Hand_Socket" "RTS_World") "Undefined" "MultiplyWithRoot" null (`self.HeldItemData`) null))
  (bind _basemesh (`BaseObject.BaseMesh` _returnvalue))
  (`PrimitiveComponent.SetSimulatePhysics` _basemesh true)
  (`SceneComponent.K2_AddWorldOffset` _basemesh (* (`self.HandleOffset`) (`SceneComponent.GetUpVector` _basemesh)) false false)
  (set `self.HoldingItem` false)
  (set `self.HeldItemData` (struct)))

(fn `GenerateProjectileInfo`
  (params (`Weapon Item Data` :type "/Game/MultiplayerLobbies/Datatables/WeaponItemData Structure") (`Gem Data` :type "Array of String"))
  (returns (`Projectile Info` :type "/Game/MultiplayerLobbies/Blueprints/DamageSystem/ProjectileInfo Structure"))
  (return))

(fn `Get Current Health`
  (returns (Health :type "Float (double-precision)"))
  (return (`/Game/MultiplayerLobbies/Blueprints/DamageSystem/BPC_DamageSystem.Health` (`self.BPC_DamageSystem`))))

(fn `Get Max Health`
  (returns (MaxHealth :type "Float (double-precision)"))
  (return (`/Game/MultiplayerLobbies/Blueprints/DamageSystem/BPC_DamageSystem.MaxHealth` (`self.BPC_DamageSystem`))))

(fn `Heal`
  (params (Amount :type "Float (double-precision)"))
  (returns (NewHealth :type "Float (double-precision)"))
  (bind _newhealth (`/Game/MultiplayerLobbies/Blueprints/DamageSystem/BPC_DamageSystem.Heal` (`self.BPC_DamageSystem`) Amount))
  (return _newhealth))

(fn `IsHoldingItem`
  (returns (HoldingItem :type Boolean))
  (return (!= (`.Name_11_B8DF43004E223A93E21556A5E1CBF881` (break `/Game/MultiplayerLobbies/Datatables/BaseItemData` (`.ItemData_2_AB890E3145ADAEB69815B3B9B749E7DE` (break `/Game/MultiplayerLobbies/Datatables/ComponentData` (`.MainBody_18_E40FCBED47D046CD11E29BA80FB2AD16` (break `/Game/MultiplayerLobbies/Datatables/WeaponItemData` (`self.HeldItemData`))))))) "Null")))

(fn `OnRep_HeldBackItemData`
  (locals (NewLocalVar :type "Array of SceneComponent Object Reference"))
  (bind _backstaffmesh (`self.BackStaffMesh`))
  (`/Game/MultiplayerLobbies/Blueprints/GenericBlueprints.DestroyAllChildren` (`self.BackStaffMesh`))
  (if (== (`.Name_11_B8DF43004E223A93E21556A5E1CBF881` (break `/Game/MultiplayerLobbies/Datatables/BaseItemData` (`.ItemData_2_AB890E3145ADAEB69815B3B9B749E7DE` (break `/Game/MultiplayerLobbies/Datatables/ComponentData` (`.MainBody_18_E40FCBED47D046CD11E29BA80FB2AD16` (break `/Game/MultiplayerLobbies/Datatables/WeaponItemData` (`self.HeldBackItemData`))))))) "Null")
    ;[1 1 1] Set To NULL
    (`StaticMeshComponent.SetStaticMesh` (`self.BackStaffMesh`) null)
    (else
      (bind _itemrowdata (`/Game/MultiplayerLobbies/Blueprints/GenericBlueprints.Construct Weapon Mesh` _backstaffmesh (`self.HeldBackItemData`) self))
      (set `self.HeldBackItemGemData` _itemrowdata)
      (`PrimitiveComponent.SetCollisionEnabled` (`self.BackStaffMesh`) "NoCollision")
      (bind _output_get (set `self.HandleOffset` (- (`SceneComponent.K2_GetComponentLocation` _backstaffmesh) (`SceneComponent.GetSocketLocation` _backstaffmesh "BackSocket"))))
      (`SceneComponent.K2_SetRelativeLocationAndRotation` :`self` _backstaffmesh :`NewLocation` (* (0.0 0.0 1.0) (`KismetMathLibrary.VSize` _output_get))))))

(fn `OnRep_HeldItemData`
  (bind _helditemmesh (`self.HeldItemMesh`))
  (`/Game/MultiplayerLobbies/Blueprints/GenericBlueprints.DestroyAllChildren` (`self.HeldItemMesh`))
  (`KismetArrayLibrary.Array_Clear` (`self.ComponentLogics`))
  (`/Game/MultiplayerLobbies/Blueprints/GenericBlueprints.DestroyAllChildren` (`self.ComponentLogic`))
  (if (== (`.Name_11_B8DF43004E223A93E21556A5E1CBF881` (break `/Game/MultiplayerLobbies/Datatables/BaseItemData` (`.ItemData_2_AB890E3145ADAEB69815B3B9B749E7DE` (break `/Game/MultiplayerLobbies/Datatables/ComponentData` (`.MainBody_18_E40FCBED47D046CD11E29BA80FB2AD16` (break `/Game/MultiplayerLobbies/Datatables/WeaponItemData` (`self.HeldItemData`))))))) "Null")
    ;[1 1 1] Set To NULL
    (`StaticMeshComponent.SetStaticMesh` (`self.HeldItemMesh`) null)
    (set `self.HoldingItem` false)
    (else
      (bind _itemrowdata (`/Game/MultiplayerLobbies/Blueprints/GenericBlueprints.Construct Weapon Mesh` _helditemmesh (`self.HeldItemData`) self (`self.ComponentLogic`)))
      (set `self.HeldItemGemData` _itemrowdata)
      (`PrimitiveComponent.SetCollisionEnabled` (`self.HeldItemMesh`) "NoCollision")
      (set `self.HoldingItem` true)
      (bind _output_get (set `self.HandleOffset` (- (`SceneComponent.K2_GetComponentLocation` _helditemmesh) (`SceneComponent.GetSocketLocation` _helditemmesh "Handle"))))
      (`SceneComponent.K2_SetRelativeLocationAndRotation` :`self` _helditemmesh :`NewLocation` (* (0.0 0.0 1.0) (`KismetMathLibrary.VSize` _output_get))))))

(fn `TakeDamage`
  (params (DamageInfo :type "/Game/MultiplayerLobbies/Blueprints/DamageSystem/DamageInfo Structure"))
  (returns (WasDamaged :type Boolean))
  (bind _wasdamaged (`/Game/MultiplayerLobbies/Blueprints/DamageSystem/BPC_DamageSystem.Take Damage` (`self.BPC_DamageSystem`) DamageInfo))
  (return _wasdamaged))

(fn `UserConstructionScript`
  (bind _bpc_damagesystem (`self.BPC_DamageSystem`))
  (add `/Game/MultiplayerLobbies/Blueprints/DamageSystem/BPC_DamageSystem.OnDeath` _bpc_damagesystem (`|CreateDelegate` :!event `Death`))
  (add `/Game/MultiplayerLobbies/Blueprints/DamageSystem/BPC_DamageSystem.OnDamageResponse` _bpc_damagesystem (`|CreateDelegate` :!event `DamageResponse`))
  (`parent.UserConstructionScript`))